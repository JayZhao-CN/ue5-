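; GI_Tcp, apparently a GameInstance, is the client hub for a TCP chat feature, linking login, message events and local history.
; It binds group and private message events on the BP_TCPBaseClass actor; private messages are only printed, group ones ignored.
; On receiving a login token, it swaps W_Login for W_Msg.
; History writing appends Base64-encoded JSON with empty fields to per-account, per-friend files under Public Documents; reading is a stub.
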(event Custom|获取到token
  ;[1 1 1] 登录成功事件
  (bind _returnvalue (UserInterface|CreateWidget "/Game/TCPCore/Widget/W_Msg.W_Msg_C"))
  (UserInterface|Viewport|AddtoViewport _returnvalue 0)
  (Widget|RemovefromParent (stale Custom|绑定登录成功事件 _output_get)))

(event Custom|收到群组消息
  (params (msg :type String) (aim :type String))
  ;[1 1 1] 收到消息事件
)

(event Custom|收到私聊消息
  (params (Msg :type String) (aim :type String))
  ;[1 1 1] 收到消息事件
  (Development|PrintString Msg))

(event Custom|绑定新消息事件
  ;[1 1 1] 收到消息事件
  (bind _outactors (Actor|GetAllActorsOfClass "/Game/TCPCore/Blueprint/BP_TCPBaseClass.BP_TCPBaseClass_C"))
  (Variables|Default|SetTCPClass (Utilities|Array|Get(acopy) _outactors))
  (Utilities|FlowControl|Sequence
    (:then_0
      (EventDispatchers|BindEventtoNewGroupMsg (Utilities|Array|Get(acopy) _outactors) (EventDispatchers|CreateEvent :!event Custom|收到群组消息)))
    (:then_1
      (EventDispatchers|BindEventtoNewPersonalMsg (Utilities|Array|Get(acopy) _outactors) (EventDispatchers|CreateEvent :!event Custom|收到私聊消息)))))

(event Custom|绑定登录成功事件
  ;[1 1 1] 登录成功事件
  (bind _foundwidgets (Widget|GetAllWidgetsOfClass "/Game/TCPCore/Widget/W_Login.W_Login_C" true))
  (bind _output_get (Variables|Default|SetLoginWidget (Utilities|Array|Get(acopy) _foundwidgets)))
  (EventDispatchers|BindEventto获取到token _output_get (EventDispatchers|CreateEvent :!event Custom|获取到token)))

(fn 读取信息
  (params (account :type String))
  (return ""))

(fn 写入本地存储文件
  (params (friendAccount :type String))
  (bind _account (Variables|Default|Getaccount))
  (bind _returnvalue (Utilities|String|Append "C:\\Users\\Public\\Documents\\UEChatRecord\\" _account "\\" friendAccount ".txt"))
  (LocalVariables|Set本地文件path _returnvalue)
  (if (.bisvalid (Class|FileSDKBPLibrary|GetFileorDirectoryInfo _returnvalue))
    _
    (else
      (Class|FileSDKBPLibrary|CreateFile (LocalVariables|Get本地文件path) true true)))
  (bind _returnvalue_2 (Class|VaRestSubsystem|ConstructVaRestJsonObject (|VaRestSubsystem)))
  (Class|VaRestJsonObject|SetStringField _returnvalue_2 "msgContent")
  (Class|VaRestJsonObject|SetStringField _returnvalue_2 "msgType")
  (Class|VaRestJsonObject|SetStringField _returnvalue_2 "msgTime")
  (Class|FileSDKBPLibrary|WriteStringtoFile (LocalVariables|Get本地文件path) (Class|VaRestLibrary|Base64Encode (Utilities|String|Append (Class|VaRestJsonObject|EncodeJson _returnvalue_2) "❤")) true "AutoDetect"))