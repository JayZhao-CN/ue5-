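; TCP chat client base actor that connects to a server and exchanges private and group messages.
; Incoming data is decoded as JSON via VaRest and routed by type: token handshake reply, group or private message dispatchers, and system notices, with friend-added notices raising their own dispatcher.
; Public send events build payloads through BPMsgHander using the GameInstance token.
; Connect and disconnect logging is left unwired.
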(event Custom|连接服务器
  (bind _connectionid (Class|TcpSocketConnection|Connect (Variables|Default|GetIp%20Address) (Variables|Default|GetPort) (EventDispatchers|CreateEvent :!event TCPMapAutoGenFunc) (EventDispatchers|CreateEvent :!event TCPMapAutoGenFunc1) (EventDispatchers|CreateEvent :!event Custom|收到消息)))
  (Variables|Default|SetConnection%20Id _connectionid))

(event Custom|发送私聊消息
  (params (msg :type String) (userId :type String))
  ;[1 1 1] 发送消息的公共接口
  (bind _returnvalue (Default|发送通用消息方法 (Variables|Default|GetBP_MsgHander) (Variables|/Game/TCPCore/Blueprint/GI_Tcp.GI_Tcp_C|Gettoken (Variables|Default|Get游戏实例)) "3" userId msg))
  (Class|TcpSocketConnection|SendData (Variables|Default|GetConnection%20Id) _returnvalue))

(event Custom|收到消息
  (params (ConnectionId :type Integer) (Message :type Array%20of%20Bytes))
  (bind _returnvalue (Class|TcpSocketConnection|MessageReadString Message (Utilities|Array|Length Message)))
  (bind (_type _msg _aim) (CallFunction|解析收到的消息 _returnvalue))
  ;[1 1 1] 初次连接发送验证token
  (if (== _type "0")
    (Class|TcpSocketConnection|SendData (Variables|Default|GetConnection%20Id) (Class|TcpSocketConnection|ToBytes(String) (Utilities|String|Append "{token:" (Variables|/Game/TCPCore/Blueprint/GI_Tcp.GI_Tcp_C|Gettoken (Variables|Default|Get游戏实例)) ",type:\"0\"}")))
    (else
      ;[1 1 1] 收到群组消息
      (if (== _type "2")
        (Default|CallNewGroupMsg _msg _aim)
        (else
          ;[1 1 1] 收到私聊消息
          (if (== _type "3")
            (Default|CallNewPersonalMsg _msg _aim)
            (elif (Utilities|Enum|Equal(Enum) _type "1")
              (if (Utilities|String|Contains _msg "已加您为好友")
                (Default|CallNewNoteMsg)
                (else
                  (Development|PrintString _msg))))))))))

(event Custom|发送群组消息
  (params (msg :type String) (groupId :type String))
  ;[1 1 1] 发送消息的公共接口
  (bind _returnvalue (Default|发送通用消息方法 (Variables|Default|GetBP_MsgHander) (Variables|/Game/TCPCore/Blueprint/GI_Tcp.GI_Tcp_C|Gettoken (Variables|Default|Get游戏实例)) "2" groupId msg))
  (Class|TcpSocketConnection|SendData (Variables|Default|GetConnection%20Id) _returnvalue))

(event EventBeginPlay
  (bind _asgi_tcp (Utilities|Casting|CastToGI_Tcp (Game|GetGameInstance)))
  (Variables|Default|Set游戏实例 _asgi_tcp))

(event Collision|EventActorBeginOverlap
  (params (OtherActor :type Actor%20Object%20Reference)))

(event EventTick
  (params (DeltaSeconds :type Float%20%28single-precision%29)))

(fn ConstructionScript)

(fn TCPMapAutoGenFunc
  (params (ConnectionId :type Integer)))

(fn TCPMapAutoGenFunc1
  (params (ConnectionId :type Integer)))

(fn 解析收到的消息
  (params (rawMsg :type String))
  (bind _returnvalue (Class|VaRestSubsystem|ConstructVaRestJsonObject (|VaRestSubsystem)))
  (Class|VaRestJsonObject|DecodeJson _returnvalue rawMsg true)
  (return (Class|VaRestJsonObject|GetStringField _returnvalue "type") (Class|VaRestJsonObject|GetStringField _returnvalue "msg") (Class|VaRestJsonObject|GetStringField _returnvalue "aim")))